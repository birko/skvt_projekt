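; BP_SkvtScreen is an in-world screen that shows a Skvt webpage widget and can be switched on, off or broken.
; On BeginPlay it caches the Webpage component's WBP_SkvtWeb widget as WebpageRef.
; Toggleon shows or hides Webpage, but a broken screen always stays off.
; Break sets the broken flag, readable through IsBroken, and switches off a screen that is on.
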(event `self.ReceiveBeginPlay`
  (`self.Initialize`))

(event `/Game/Skvt/Blueprints/BPI_Electric.Break`
  (set `self.BrokenStatus` true)
  (if (`self.IsOn`)
    (`/Game/Skvt/Blueprints/BPI_Electric.ToggleON` false)))

(event `/Game/Skvt/Blueprints/BPI_Electric.ToggleOn`
  (params (IsOn :type Boolean))
  (bind _output_get (set `self.IsOn` (and IsOn (not (`self.BrokenStatus`)))))
  (`SceneComponent.SetVisibility` (`self.Webpage`) _output_get false))

(fn `Initialize`
  (bind _aswbp_skvt_web (cast `/Game/Skvt/Blueprints/Screen/WBP_SkvtWeb` (`WidgetComponent.GetWidget` (`self.Webpage`))))
  (set `self.WebpageRef` _aswbp_skvt_web))

(fn `IsBroken`
  (returns (IsBroken :type Boolean))
  (return (`self.BrokenStatus`)))

(fn `UserConstructionScript`)